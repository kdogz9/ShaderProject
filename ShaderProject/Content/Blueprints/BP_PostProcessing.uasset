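; BP_PostProcessing applies the M_PostProcess material to its Camera as a post-process blendable.
; On BeginPlay it enables player input, creates a dynamic material instance and writes it into the camera's post-process settings at the current Weight.
; The F key flip-flops Weight between on and off values, but nothing writes the new value back to the camera settings after BeginPlay.
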(event EventBeginPlay
  (Input|EnableInput (Game|GetPlayerController 0))
  (bind _returnvalue (Rendering|Material|CreateDynamicMaterialInstance "/Game/Materials/M_PostProcess.M_PostProcess" "None" "None" :!class /Script/Engine.KismetMaterialLibrary))
  (Variables|/Script/Engine.CameraComponent|SetPostProcessSettings (Variables|Default|GetCamera) (Utilities|Struct|MakePostProcessSettings (Utilities|Struct|MakeWeightedBlendables (Utilities|Array|MakeArray (Utilities|Struct|MakeWeightedBlendable (Variables|Default|GetWeight) _returnvalue))))))

(event Input|KeyboardEvents|F
  (params (Key :type Key%20Structure :default "None"))
  (:Pressed
    (Utilities|FlowControl|FlipFlop
      (:A
        (Variables|Default|SetWeight 1.0))
      (:B
        (Variables|Default|SetWeight 0.0)))))

(fn ConstructionScript)