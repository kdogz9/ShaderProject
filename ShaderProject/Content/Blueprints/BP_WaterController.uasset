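; BP_WaterController is an actor that recolors its water mesh at runtime in response to a key press.
; On BeginPlay it enables input from the first player controller and puts a dynamic material instance on WaterMesh.
; Pressing the 1 key sets that instance's WaterTint parameter to a fixed pink and prints a debug string.
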(event EventBeginPlay
  (Input|EnableInput (Game|GetPlayerController 0))
  (bind _returnvalue (Rendering|Material|CreateDynamicMaterialInstance (Variables|Default|GetWaterMesh) 0 0 "None" :!class /Script/Engine.PrimitiveComponent))
  (bind _output_get (Variables|Default|SetDMI_Water _returnvalue))
  (Rendering|Material|SetMaterial (Variables|Default|GetWaterMesh) 0 _output_get))

(event Input|KeyboardEvents|1
  (params (Key :type Key%20Structure :default "None"))
  (:Pressed
    (Rendering|Material|SetVectorParameterValue (Variables|Default|GetDMI_Water) "WaterTint" "(R=1.000000,G=0.004179,B=0.355707,A=1.000000)" :!class /Script/Engine.MaterialInstanceDynamic)
    (Development|PrintString "Hello")))

(fn ConstructionScript)