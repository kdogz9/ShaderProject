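; BP_Glow is an actor with an Orb mesh whose glowing material can be changed at runtime by key presses.
; On BeginPlay it enables input from the first player controller and applies a dynamic instance of M_Glow to the Orb.
; The 3 key sets a high GlowStrength on that instance, and the 2 key lowers OpacityLevel to make the orb more transparent.
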(event EventBeginPlay
  (Input|EnableInput (Game|GetPlayerController 0))
  (bind _returnvalue (Rendering|Material|CreateDynamicMaterialInstance (Variables|Default|GetOrb) 0 "/Game/Materials/M_Glow.M_Glow" "None" :!class /Script/Engine.PrimitiveComponent))
  (bind _output_get (Variables|Default|SetDMI_Orb _returnvalue))
  (Rendering|Material|SetMaterial (Variables|Default|GetOrb) 0 _output_get))

(event Input|KeyboardEvents|2
  (params (Key :type Key%20Structure :default "None"))
  (:Pressed
    (Rendering|Material|SetScalarParameterValue (Variables|Default|GetDMI_Orb) "OpacityLevel" 0.2 :!class /Script/Engine.MaterialInstanceDynamic)))

(event Input|KeyboardEvents|3
  (params (Key :type Key%20Structure :default "None"))
  (:Pressed
    (Rendering|Material|SetScalarParameterValue (Variables|Default|GetDMI_Orb) "GlowStrength" 5e+03 :!class /Script/Engine.MaterialInstanceDynamic)))

(fn ConstructionScript)